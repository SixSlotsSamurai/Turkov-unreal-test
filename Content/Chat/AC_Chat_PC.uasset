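; Chat component for a PlayerController that shows a chat UI and relays messages to all players.
; On BeginPlay, the local controller creates the WB_ChatUI widget and caches its chat box, which Enter focuses and the mouse wheel scrolls.
; SendChatMessage loops through the GameState PlayerArray and calls AddChatMessageOnOwningClient on each controller's chat component, which appends the text to that player's chat box.
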(event `self.ReceiveBeginPlay`
  (if (`Controller.IsLocalPlayerController` (cast `PlayerController` (`self.GetOwner`) :!pure true))
    (bind _returnvalue (`|CreateWidget` "/Game/Chat/WB_ChatUI.WB_ChatUI_C"))
    (bind _output_get (set `self.ChatUI_Ref` _returnvalue))
    (`UserWidget.AddToViewport` _output_get 0)
    (set `self.WBChatBox_Ref` (`/Game/Chat/WB_ChatUI.WB_ChatBox` _output_get))))

(event `Key|Enter`
  (params (Key :type "Key Structure"))
  (:`Pressed`
    (`/Game/Chat/WB_ChatBox.Focus` (`self.WBChatBox_Ref`))))

(event `Key|MouseScrollUp`
  (params (Key :type "Key Structure"))
  (:`Pressed`
    (`/Game/Chat/WB_ChatBox.Scroll` (`self.WBChatBox_Ref`) true)))

(event `Key|MouseScrollDown`
  (params (Key :type "Key Structure"))
  (:`Pressed`
    (`/Game/Chat/WB_ChatBox.Scroll` (`self.WBChatBox_Ref`) false)))

(event `SendChatMessage`
  (params (Message :type String))
  (for _array_element (`GameStateBase.PlayerArray` (`GameplayStatics.GetGameState`))
    (`self.AddChatMessageOnOwningClient` (`Actor.K2_GetComponentsByClass` (`PlayerState.GetPlayerController` _array_element) "AC_Chat_PC_C") Message)))

(event `AddChatMessageOnOwningClient`
  (params (Message :type String))
  (`/Game/Chat/WB_ChatBox.AddChatMessage` (`self.WBChatBox_Ref`) Message))